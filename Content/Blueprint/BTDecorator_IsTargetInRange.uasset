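; Behavior Tree decorator that checks whether the AI's target is within range of its controlled pawn.
; It reads the Target actor from the Blackboard and compares the distance between the pawn and that actor against Range.
; When in range it prints a Korean "found it" debug message and returns true; the out-of-range branch has no explicit return.
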(fn `PerformConditionCheckAI`
  (params (OwnerController :type "AIController Object Reference") (ControlledPawn :type "Pawn Object Reference"))
  (returns (ReturnValue :type Boolean))
  (bind _returnvalue (<= (`KismetMathLibrary.VSize` (- (`Actor.K2_GetActorLocation` ControlledPawn) (`Actor.K2_GetActorLocation` (`BTFunctionLibrary.GetBlackboardValueAsActor` (`self.Target`))))) (`self.Range`)))
  (if _returnvalue
    (`KismetSystemLibrary.PrintText` "찾았다")
    (return _returnvalue)))