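; BP_Player is the player character Blueprint, handling weapon firing and debug logging of capsule collisions.
; FireWeapon plays a fire montage, then deprojects a point slightly above screen center and traces along it to find the aim location.
; A second trace runs from the mesh's GunSocket to that hit location; both only draw debug lines, with no damage applied.
; Capsule hit and overlap events, plus an Iscreated function, just print messages.
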(event `self.CapsuleComponent.OnComponentHit`
  (params (HitComponent :type "PrimitiveComponent Object Reference") (OtherActor :type "Actor Object Reference") (OtherComp :type "PrimitiveComponent Object Reference") (NormalImpulse :type "Vector Structure") (Hit :type "HitResult Structure (by ref)"))
  (`KismetSystemLibrary.PrintText` "Player Hit"))

(event `self.CapsuleComponent.OnComponentBeginOverlap`
  (params (OverlappedComponent :type "PrimitiveComponent Object Reference") (OtherActor :type "Actor Object Reference") (OtherComp :type "PrimitiveComponent Object Reference") (OtherBodyIndex :type Integer) (bFromSweep :type Boolean) (SweepResult :type "HitResult Structure (by ref)"))
  (`KismetSystemLibrary.PrintText` "Player BeginOverlap"))

(event `self.CapsuleComponent.OnComponentEndOverlap`
  (params (OverlappedComponent :type "PrimitiveComponent Object Reference") (OtherActor :type "Actor Object Reference") (OtherComp :type "PrimitiveComponent Object Reference") (OtherBodyIndex :type Integer))
  (`KismetSystemLibrary.PrintText` "Player EndOverlap"))

(fn `FireWeapon`
  (bind (_returnvalue_x _returnvalue_y) (`KismetMathLibrary.BreakVector2D` (`WidgetLayoutLibrary.GetViewportSize`)))
  (bind _returnvalue_location (`KismetMathLibrary.BreakTransform` (`SceneComponent.GetSocketTransform` (`self.Mesh`) "GunSocket" "RTS_World")))
  (bind (_worldposition _worlddirection _returnvalue) (`GameplayStatics.DeprojectScreenToWorld` (`GameplayStatics.GetPlayerController` 0) (`KismetMathLibrary.MakeVector2D` (/ _returnvalue_x 2.0) (- (/ _returnvalue_y 2.0) 50.0))))
  (`self.PlayAnimMontage` "/Game/Animations/AM_Fire.AM_Fire" 1.0 "Start")
  (if _returnvalue
    (bind _outhit (`KismetSystemLibrary.LineTraceSingle` :`Start` _worldposition :`End` (+ _worldposition (* _worlddirection 5000.0)) :`TraceChannel` "TraceTypeQuery1" :`DrawDebugType` "ForDuration" :`DrawTime` 1.0))
    (`KismetSystemLibrary.LineTraceSingle` :`Start` _returnvalue_location :`End` (`.Location` (`GameplayStatics.BreakHitResult` _outhit)) :`TraceChannel` "TraceTypeQuery1" :`DrawDebugType` "ForDuration" :`DrawTime` 1.0)))

(fn `iscreated`
  (`KismetSystemLibrary.PrintText` "만들어졌다"))

(fn `UserConstructionScript`)