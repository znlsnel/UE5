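; BP_Plane is a simple flyable plane that constantly moves forward and is steered by player input.
; Tick advances the actor along its forward vector at MoveSpeed, scaled by delta time and without sweeping for collision.
; The XTurn and Yturn axes share one local rotation of the root, applying roll and pitch from axis input, RotateSpeed and delta time, with no yaw.
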(event `self.ReceiveTick`
  (params (DeltaSeconds :type "Float (single-precision)"))
  (`self.K2_SetActorLocation` (+ (`self.K2_GetActorLocation`) (* (`self.GetActorForwardVector`) (`self.MoveSpeed`) DeltaSeconds))))

(event `InputAxis|XTurn`
  (params (AxisValue :type "Float (single-precision)"))
  (if (!= AxisValue 0.0)
    (`SceneComponent.K2_AddLocalRotation` (`self.DefaultSceneRoot`) (`KismetMathLibrary.MakeRotator` (* AxisValue (`self.RotateSpeed`) (`GameplayStatics.GetWorldDeltaSeconds`)) (* (stale `InputAxis|Yturn` AxisValue) (`GameplayStatics.GetWorldDeltaSeconds`) (`self.RotateSpeed`))) false false :!label _label)))

(event `InputAxis|Yturn`
  (params (AxisValue :type "Float (single-precision)"))
  (if (!= AxisValue 0.0)
    (goto _label)))

(fn `UserConstructionScript`)