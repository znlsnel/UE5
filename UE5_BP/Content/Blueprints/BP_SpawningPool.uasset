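; BP_SpawningPool keeps a BP_Tilemap owner populated with BP_Skeleton creatures up to a maximum count.
; On BeginPlay it caches the owning tilemap and starts a self-calling spawn loop.
; Below the cap, the loop reserves a slot, waits a short random delay, then asks the tilemap to spawn; at the cap it rechecks each tick.
; OnDespawnCreature decrements the count, freeing a slot for a replacement.
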(event `self.ReceiveBeginPlay`
  (bind _asbp_tilemap (cast `/Game/Blueprints/BP_Tilemap` (`self.GetOwner`)))
  (set `self.Tilemap` _asbp_tilemap)
  (`self.UpdateRandomSpawn`))

(event `UpdateRandomSpawn`
  (if (< (`self.CreatureCount`) (`self.MaxCreatureCount`))
    (`/Engine/EditorBlueprintResources/StandardMacros.IncrementInt` (`self.CreatureCount`)
      (:`  `
        (`KismetSystemLibrary.Delay` (`KismetMathLibrary.RandomFloatInRange` 2.0 5.0))
        (`/Game/Blueprints/BP_Tilemap.SpawnCreature` (`self.Tilemap`) "/Game/Blueprints/Creatures/BP_Skeleton.BP_Skeleton_C")))
    (else
      (`KismetSystemLibrary.DelayUntilNextTick`)))
  (`self.UpdateRandomSpawn`))

(fn `OnDespawnCreature`
  (`/Engine/EditorBlueprintResources/StandardMacros.DecrementInt` (`self.CreatureCount`)))