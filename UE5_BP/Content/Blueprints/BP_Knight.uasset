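; BP_Knight is a sprite-based knight that animates idle, move and attack in four facing directions.
; Each tick it derives State and Direction from the movement axes, with horizontal input overriding vertical, then picks the matching flipbook.
; Left reuses the side flipbooks by rotating the sprite 180 degrees.
; Attack holds the Skill state for the flipbook's length, blocking state but not direction changes, then returns to Move.
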(event `self.ReceiveTick`
  (params (DeltaSeconds :type "Float (single-precision)"))
  (`self.UpdateInput`)
  (`self.Update Animation`))

(event `InputAction|Attack`
  (params (Key :type "Key Structure"))
  (:`Pressed`
    (set `self.State` "NewEnumerator2")
    (`self.Update Animation`)
    (`KismetSystemLibrary.Delay` (`PaperFlipbookComponent.GetFlipbookLength` (`self.Sprite`)))
    (set `self.State` "NewEnumerator1")))

(fn `Update Animation`
  (`SceneComponent.K2_SetRelativeRotation` (`self.Sprite`) (select `bool` (`|EnumEquality` (`self.Direction`) "NewEnumerator2") :`false` (struct) :`true` (struct :`Yaw` 180.0) :!type "Rotator Structure") false false)
  (switch `/Game/Blueprints/EState` (`self.State`)
    (:`NewEnumerator0`
      (`PaperFlipbookComponent.SetFlipbook` (`self.Sprite`) (select `/Game/Blueprints/EDirection` (`self.Direction`) :`NewEnumerator0` "/Game/Maps/Sprite/Player/Knight/up_idle.up_idle" :`NewEnumerator1` "/Game/Maps/Sprite/Player/Knight/down_idle.down_idle" :`NewEnumerator2` "/Game/Maps/Sprite/Player/Knight/side_idle.side_idle" :`NewEnumerator3` "/Game/Maps/Sprite/Player/Knight/side_idle.side_idle" :!type "PaperFlipbook Object Reference")))
    (:`NewEnumerator1`
      (`PaperFlipbookComponent.SetFlipbook` (`self.Sprite`) (select `/Game/Blueprints/EDirection` (`self.Direction`) :`NewEnumerator0` "/Game/Maps/Sprite/Player/Knight/up_move.up_move" :`NewEnumerator1` "/Game/Maps/Sprite/Player/Knight/down_move.down_move" :`NewEnumerator2` "/Game/Maps/Sprite/Player/Knight/side_move.side_move" :`NewEnumerator3` "/Game/Maps/Sprite/Player/Knight/side_move.side_move" :!type "PaperFlipbook Object Reference")))
    (:`NewEnumerator2`
      (`PaperFlipbookComponent.SetFlipbook` (`self.Sprite`) (select `/Game/Blueprints/EDirection` (`self.Direction`) :`NewEnumerator0` "/Game/Maps/Sprite/Player/Knight/up_attack.up_attack" :`NewEnumerator1` "/Game/Maps/Sprite/Player/Knight/down_attack.down_attack" :`NewEnumerator2` "/Game/Maps/Sprite/Player/Knight/side_attack.side_attack" :`NewEnumerator3` "/Game/Maps/Sprite/Player/Knight/side_attack.side_attack" :!type "PaperFlipbook Object Reference")))))

(fn `UpdateInput`
  (`|ExecutionSequence`
    (:`then_0`
      (if (`|EnumEquality` (`self.State`) "NewEnumerator2")
        _
        (elif (or (!= (`self.GetInputAxisValue`) 0.0) (!= (`self.GetInputAxisValue`) 0.0))
          (set `self.State` "NewEnumerator1")
          (else
            (set `self.State` "NewEnumerator0")))))
    (:`then_1`
      (`/Engine/EditorBlueprintResources/StandardMacros.CompareFloat` (`self.GetInputAxisValue`)
        (:`>`
          (set `self.Direction` "NewEnumerator0"))
        (:`<`
          (set `self.Direction` "NewEnumerator1"))))
    (:`then_2`
      (`/Engine/EditorBlueprintResources/StandardMacros.CompareFloat` (`self.GetInputAxisValue`)
        (:`>`
          (set `self.Direction` "NewEnumerator3"))
        (:`<`
          (set `self.Direction` "NewEnumerator2"))))))

(fn `UserConstructionScript`)